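; Gameplay game mode for the Crossy Road game that sets up references and the gameplay camera on BeginPlay.
; It caches the player character and every vehicle derived from BP_VehicleParent, stopping that branch if the player cast fails.
; It then disables player input and spawns a camera actor at the stored gameplay location and rotation, blending the view to it over a few seconds.
; Input is not re-enabled in this Blueprint.
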(event EventBeginPlay
  (Utilities|FlowControl|Sequence
    (:then_0
      ;[0 1 0] Reference to Player
      (bind _asbp_player (Utilities|Casting|CastToBP_Player (Game|GetPlayerCharacter 0)))
      (Variables|References|SetPlayer_Ref _asbp_player)
      ;[0 1 0] Reference to all enemies
      (bind _outactors (Actor|GetAllActorsOfClass "/Game/Crossy_Road/Blueprints/Characters/BP_VehicleParent.BP_VehicleParent_C"))
      (Variables|References|SetVehicles _outactors))
    (:then_3
      (Input|DisableInput (Game|GetPlayerCharacter 0) (Game|GetPlayerController 0))
      (bind _returnvalue (Game|SpawnActorfromClass "/Script/Engine.CameraActor" (Math|Transform|MakeTransform (Variables|Camera|GetCamGameplay_Loc) (Variables|Camera|GetCamGameplay_Rot) "1,1,1") "Undefined" 0 0))
      (Game|Player|SetViewTargetwithBlend (Game|GetPlayerController 0) _returnvalue 3.5 "VTBlend_Linear" 0.0 false))))

(fn ConstructionScript)